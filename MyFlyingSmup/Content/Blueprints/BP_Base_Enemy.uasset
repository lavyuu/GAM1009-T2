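; Base enemy actor that damages any actor overlapping it by an amount equal to its current Health.
; Damage taken is sent to the player controller as score, lowers clamped Health, updates the health widget through messages, plays a sound and briefly flashes a hit overlay material.
; At zero Health it plays a sound, spawns a Niagara explosion and its configured pickup, then destroys itself.
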(event `self.ReceiveBeginPlay`
  (set `self.Health` (`self.Health`)))

(event `self.ReceiveActorBeginOverlap`
  (params (OtherActor :type "Actor Object Reference"))
  (`GameplayStatics.ApplyDamage` OtherActor (`self.Health`)))

(event `self.ReceiveAnyDamage`
  (params (Damage :type "Float (single-precision)") (DamageType :type "DamageType Object Reference") (InstigatedBy :type "Controller Object Reference") (DamageCauser :type "Actor Object Reference"))
  (message `/Game/core/BPI_MyFlyingShmup.AddScore` (`GameplayStatics.GetPlayerController` 0) Damage)
  (set `self.Health` (`KismetMathLibrary.FClamp` (- (`self.Health`) Damage) 0.0 (`self.MaxHealth`)))
  (message `/Game/core/BPI_MyFlyingShmup.SetHealthPercent` (`WidgetComponent.GetUserWidgetObject` (`self.Widget`)) (`KismetMathLibrary.SafeDivide` (`self.Health`) (`self.MaxHealth`)))
  (`self.CheckHealth`)
  (`GameplayStatics.PlaySound2D` "/Game/FreeModularMagicSFX/E_Impact/Mono/SW_MagicImpact_Fire_3.SW_MagicImpact_Fire_3" 1.0 1.0 0.0 null null)
  (`self.FlashRedOverlayMaterial`))

(event `CheckHealth`
  (if (== (`self.Health`) 0.0)
    (message `/Game/core/BPI_MyFlyingShmup.AddScore` (`GameplayStatics.GetPlayerController` 0) 0.0)
    (`self.OnDeath`)))

(event `OnDeath`
  (bind (_returnvalue_location _returnvalue_rotation) (`KismetMathLibrary.BreakTransform` (`self.GetTransform`)))
  (`GameplayStatics.PlaySound2D` "/Game/FreeModularMagicSFX/E_Impact/Mono/SW_MagicImpact_Fire_3.SW_MagicImpact_Fire_3" 1.0 1.0 0.0 null null)
  (`self.SpawnExplosion`)
  (`|SpawnActorFromClass` (`self.PickUpToDropOnDeath`) (`KismetMathLibrary.MakeTransform` _returnvalue_location _returnvalue_rotation) "Undefined" "MultiplyWithRoot" null null)
  (`self.K2_DestroyActor`))

(event `FlashRedOverlayMaterial`
  (bind _mesh (`self.Mesh`)
    (:`then`
      (`MeshComponent.SetOverlayMaterial` _mesh "/Game/Materials/M_OverlayWhenHit.M_OverlayWhenHit")
      (`KismetSystemLibrary.Delay` 0.2)
      (bind _mesh_2 (`self.Mesh`)
        (:`then`
          (`MeshComponent.SetOverlayMaterial` _mesh_2 null))
        (:`else`)))
    (:`else`)))

(event `SpawnExplosion`
  (`NiagaraFunctionLibrary.SpawnSystemAtLocation` "/Game/Particles/FX_EnemyExplosion_System.FX_EnemyExplosion_System" (`self.K2_GetActorLocation`)))

(fn `UserConstructionScript`)