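; Enemy spawner actor that periodically spawns BP_Enemy_A along a line between its left and right arrow components.
; A timer with a random delay of a few seconds triggers each spawn, then re-queues itself for an endless, irregular cadence.
; Each enemy takes a random Y between the two arrows, with X, Z and rotation copied from the left arrow.
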(event `self.ReceiveBeginPlay`
  (`self.QueueTimer`))

(event `QueueTimer`
  (`KismetSystemLibrary.K2_SetTimerDelegate` (delegate `SpawnEnemy`) (`KismetMathLibrary.RandomFloatInRange` 2.0 6.0)))

(event `SpawnEnemy`
  (bind _arrowleft (`self.ArrowLeft`))
  (bind (_returnvalue_x _returnvalue_y _returnvalue_z) (`KismetMathLibrary.BreakVector` (`SceneComponent.K2_GetComponentLocation` _arrowleft)))
  (bind (_returnvalue_x_2 _returnvalue_y_2) (`KismetMathLibrary.BreakVector` (`SceneComponent.K2_GetComponentLocation` (`self.ArrowRight`))))
  (`|SpawnActorFromClass` "/Game/Blueprints/BP_Enemy_A.BP_Enemy_A_C" (`KismetMathLibrary.MakeTransform` (`KismetMathLibrary.MakeVector` _returnvalue_x (`KismetMathLibrary.RandomFloatInRange` _returnvalue_y _returnvalue_y_2) _returnvalue_z) (`SceneComponent.K2_GetComponentRotation` _arrowleft)) "Undefined" "MultiplyWithRoot" null null)
  (`self.QueueTimer`))

(fn `UserConstructionScript`)