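; Enemy actor that shoots bullets, takes damage and drops a pickup when destroyed.
; BeginPlay sets a timer that spawns an enemy 2D bullet from its Arrow component.
; Damage lowers clamped health, updates the health widget, messages the player controller's score, plays a sound and briefly flashes a hit overlay material across its meshes.
; At zero health it sends another score message, spawns a Niagara explosion and the pickup, then destroys itself.
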(event `self.ReceiveAnyDamage`
  (params (Damage :type "Float (single-precision)") (DamageType :type "DamageType Object Reference") (InstigatedBy :type "Controller Object Reference") (DamageCauser :type "Actor Object Reference"))
  (message `/Game/core/BPI_MyFlyingShmup.AddScore` (`GameplayStatics.GetPlayerController` 0) 0.0)
  (set `self.Health` (`KismetMathLibrary.FClamp` (- (`self.Health`) Damage) 0.0 (`self.MaxHealth`)))
  (message `/Game/core/BPI_MyFlyingShmup.SetHealthPercent` (`WidgetComponent.GetUserWidgetObject` (`self.Widget`)) (`KismetMathLibrary.SafeDivide` (`self.Health`) (`self.MaxHealth`)))
  (`self.CheckHealth`)
  (`GameplayStatics.PlaySound2D` "/Game/FreeModularMagicSFX/E_Impact/Mono/SW_MagicImpact_Fire_3.SW_MagicImpact_Fire_3" 1.0 1.0 0.0 null null)
  (`self.FlashRedOverlayMaterial`))

(event `self.ReceiveBeginPlay`
  (`self.BeginRegularShooting`))

(event `BeginRegularShooting`
  (`KismetSystemLibrary.K2_SetTimerDelegate` (delegate `SpawnBullet`) 2.0))

(event `self.CheckHealth`
  (if (== (`self.Health`) 0.0)
    (message `/Game/core/BPI_MyFlyingShmup.AddScore` (`GameplayStatics.GetPlayerController` 0) 0.0)
    (`self.OnDeath`)))

(event `self.OnDeath`
  (bind (_returnvalue_location _returnvalue_rotation) (`KismetMathLibrary.BreakTransform` (`self.GetTransform`)))
  (`GameplayStatics.PlaySound2D` "/Game/FreeModularMagicSFX/E_Impact/Mono/SW_MagicImpact_Fire_3.SW_MagicImpact_Fire_3" 1.0 1.0 0.0 null null)
  (`self.SpawnExplosion`)
  (`|SpawnActorFromClass` (`self.PickUpToDropOnDeath`) (`KismetMathLibrary.MakeTransform` _returnvalue_location _returnvalue_rotation) "Undefined" "MultiplyWithRoot" null null)
  (`self.K2_DestroyActor`))

(event `SpawnBullet`
  (bind (_returnvalue_location _returnvalue_rotation) (`KismetMathLibrary.BreakTransform` (`SceneComponent.K2_GetComponentToWorld` (`self.Arrow`))))
  (`|SpawnActorFromClass` "/Game/Blueprints/BP_2DBullet_Enemy.BP_2DBullet_Enemy_C" (`KismetMathLibrary.MakeTransform` _returnvalue_location _returnvalue_rotation) "Undefined" "MultiplyWithRoot" null null))

(event `self.FlashRedOverlayMaterial`
  (bind _mesh (`self.Mesh`)
    (:`then`
      (`MeshComponent.SetOverlayMaterial` _mesh "/Game/Materials/M_OverlayWhenHit.M_OverlayWhenHit")
      (`MeshComponent.SetOverlayMaterial` (`self.Cylinder1`) "/Game/Materials/M_OverlayWhenHit.M_OverlayWhenHit")
      (`MeshComponent.SetOverlayMaterial` (`self.Cylinder2`) "/Game/Materials/M_OverlayWhenHit.M_OverlayWhenHit")
      (`MeshComponent.SetOverlayMaterial` (`self.Cylinder`) "/Game/Materials/M_OverlayWhenHit.M_OverlayWhenHit")
      (`KismetSystemLibrary.Delay` 0.2)
      (bind _mesh_2 (`self.Mesh`)
        (:`then`
          (`MeshComponent.SetOverlayMaterial` _mesh_2 null)
          (`MeshComponent.SetOverlayMaterial` (`self.Cylinder1`) null)
          (`MeshComponent.SetOverlayMaterial` (`self.Cylinder2`) null)
          (`MeshComponent.SetOverlayMaterial` (`self.Cylinder`) null))
        (:`else`)))
    (:`else`)))

(event `self.SpawnExplosion`
  (`NiagaraFunctionLibrary.SpawnSystemAtLocation` "/Game/Particles/FX_EnemyExplosion_System.FX_EnemyExplosion_System" (`self.K2_GetActorLocation`)))

(fn `UserConstructionScript`
  (`parent.UserConstructionScript`))