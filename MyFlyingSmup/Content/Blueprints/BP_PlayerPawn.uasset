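; Player pawn for a flying shmup: moves via FloatingPawnMovement and Enhanced Input, with two seconds of spawn collision immunity.
; Primary fire waits briefly, then spawns a yaw-fanned spray of bullets.
; Damage triggers camera shake, red overlay flash and health check, which updates the HUD and reports death to the controller with an explosion.
; Overlaps deal current Health as damage; pickups add health, max health and lives.
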(event `self.ReceiveBeginPlay`
  (`PrimitiveComponent.SetCollisionEnabled` (`self.Sphere`) "NoCollision")
  (`KismetSystemLibrary.Delay` 2.0)
  (`PrimitiveComponent.SetCollisionEnabled` (`self.Sphere`) "QueryAndPhysics"))

(event `self.ReceiveActorBeginOverlap`
  (params (OtherActor :type "Actor Object Reference"))
  ; Damage System
  (`GameplayStatics.ApplyDamage` OtherActor (`self.Health`)))

(event `EnhancedInput|/Game/Inputs/IA_PrimaryFire`
  (params (ActionValue :type Boolean) (ElapsedSeconds :type "Float (double-precision)") (TriggeredSeconds :type "Float (double-precision)") (InputAction :type "InputAction Object Reference" :default "/Game/Inputs/IA_PrimaryFire.IA_PrimaryFire"))
  (bind _primaryfirespawnpoint (`self.PrimaryFireSpawnPoint`))
  (bind (_returnvalue_roll _returnvalue_pitch _returnvalue_yaw) (`KismetMathLibrary.BreakRotator` (`KismetMathLibrary.MakeRotFromX` (`SceneComponent.GetForwardVector` _primaryfirespawnpoint))))
  ; Shooing
  (:`Triggered`
    (`KismetSystemLibrary.Delay` 0.2)
    ;; Shooting Mode 2
    (for _index (range 1 (+ (`self.NumberOfBulletsToSpray`) 1))
      (`|SpawnActorFromClass` "/Game/Blueprints/BP_2DBullet_Player.BP_2DBullet_Player_C" (`KismetMathLibrary.MakeTransform` (`SceneComponent.K2_GetComponentLocation` _primaryfirespawnpoint) (`KismetMathLibrary.MakeRotator` _returnvalue_roll _returnvalue_pitch (+ _returnvalue_yaw (- (* _index (`self.AngleOfSprayBullets`)) (* (`KismetMathLibrary.Round` (* (`self.NumberOfBulletsToSpray`) 0.5)) (`self.AngleOfSprayBullets`)))))) "Undefined" "MultiplyWithRoot" null null)
      (`GameplayStatics.PlaySound2D` "/Game/FreeModularMagicSFX/C_Cast/Mono/SW_MagicCast_Generic1_1.SW_MagicCast_Generic1_1" 1.0 1.0 0.0 null null))))

(event `self.ReceivePossessed`
  (params (NewController :type "Controller Object Reference"))
  (bind _asplayer_controller (cast `PlayerController` NewController))
  (bind _output_get (set `self.As Player Controller` _asplayer_controller))
  (`EnhancedInputSubsystemInterface.AddMappingContext` (pcsubsystem `EnhancedInputLocalPlayerSubsystem` _output_get) "/Game/Inputs/IMC_PlayerInputs.IMC_PlayerInputs" 0 (struct)))

(event `self.ReceiveAnyDamage`
  (params (Damage :type "Float (single-precision)") (DamageType :type "DamageType Object Reference") (InstigatedBy :type "Controller Object Reference") (DamageCauser :type "Actor Object Reference"))
  ; Damage System
  (set `self.Health` (`KismetMathLibrary.FClamp` (- (`self.Health`) Damage) 0.0 (`self.MaxHealth`)))
  (`self.ApplyCameraShake`)
  (`self.FlashRedOverlayMaterial`)
  (`self.CheckHealth`))

(event `CheckHealth`
  ; Damage System
  (message `/Game/core/BPI_MyFlyingShmup.SetHealthPercent` (`PlayerController.GetHUD` (`self.GetLocalViewingPlayerController`)) (`KismetMathLibrary.SafeDivide` (`self.Health`) (`self.MaxHealth`)))
  (`self.UpdateHUD`)
  (if (== (`self.Health`) 0.0)
    (`self.OnDeath`)))

(event `EnhancedInput|/Game/Inputs/IA_MoveForwardBackward`
  (params (ActionValue :type "Float (double-precision)") (ElapsedSeconds :type "Float (double-precision)") (TriggeredSeconds :type "Float (double-precision)") (InputAction :type "InputAction Object Reference" :default "/Game/Inputs/IA_MoveForwardBackward.IA_MoveForwardBackward"))
  ; Movement
  (:`Triggered`
    (`PawnMovementComponent.AddInputVector` (`self.FloatingPawnMovement`) (* ActionValue (`self.GetActorForwardVector`)) false)))

(event `EnhancedInput|/Game/Inputs/IA_MoveRightLeft`
  (params (ActionValue :type "Float (double-precision)") (ElapsedSeconds :type "Float (double-precision)") (TriggeredSeconds :type "Float (double-precision)") (InputAction :type "InputAction Object Reference" :default "/Game/Inputs/IA_MoveRightLeft.IA_MoveRightLeft"))
  ; Movement
  (:`Triggered`
    (`PawnMovementComponent.AddInputVector` (`self.FloatingPawnMovement`) (* ActionValue (`self.GetActorRightVector`)) false)))

(event `FlashRedOverlayMaterial`
  ; Damage System
  (`MeshComponent.SetOverlayMaterial` (`self.Mesh`) "/Game/Materials/M_OverlayWhenHit.M_OverlayWhenHit")
  (`MeshComponent.SetOverlayMaterial` (`self.Cylinder`) "/Game/Materials/M_OverlayWhenHit.M_OverlayWhenHit")
  (`MeshComponent.SetOverlayMaterial` (`self.Cone1`) "/Game/Materials/M_OverlayWhenHit.M_OverlayWhenHit")
  (`MeshComponent.SetOverlayMaterial` (`self.Cone`) "/Game/Materials/M_OverlayWhenHit.M_OverlayWhenHit")
  (`KismetSystemLibrary.Delay` 0.2)
  (`MeshComponent.SetOverlayMaterial` (`self.Mesh`) null)
  (`MeshComponent.SetOverlayMaterial` (`self.Cone`) null)
  (`MeshComponent.SetOverlayMaterial` (`self.Cone1`) null)
  (`MeshComponent.SetOverlayMaterial` (`self.Cylinder`) null))

(event `OnDeath`
  ; Damage System
  (message `/Game/core/BPI_MyFlyingShmup.OnPlayerDeath` (`self.GetController`))
  (`NiagaraFunctionLibrary.SpawnSystemAtLocation` "/Game/Particles/FX_PlayerExplosion_System.FX_PlayerExplosion_System" (`self.K2_GetActorLocation`)))

(event `/Game/core/BPI_MyFlyingShmup.OnPickUp`
  (params (AddMaxHealth :type "Float (double-precision)") (AddHealth :type "Float (double-precision)") (AddLives :type Integer) (SetMaxLivesLimit :type Integer) (AddScore :type Integer) (SetShootingModeIndez :type Integer) (AddShootingModeIndex :type Integer))
  ; Pick up system
  (`|ExecutionSequence`
    (:`then_0`
      (set `self.MaxHealth` (+ AddMaxHealth (`self.MaxHealth`))))
    (:`then_1`
      (set `self.Health` (`KismetMathLibrary.FClamp` (+ AddHealth (`self.Health`)) 0.0 (`self.MaxHealth`)))
      (`self.CheckHealth`)
      (message `/Game/core/BPI_MyFlyingShmup.AddPlayerLives` (`self.GetController`) AddLives))))

(event `ApplyCameraShake`
  ; Damage System
  (`GameplayStatics.PlayWorldCameraShake` "/Game/Blueprints/BP_CameraShake.BP_CameraShake_C" (0.0 0.0 0.0) 0.0 10000.0))

(event `UpdateHUD`
  ; Damage System
  (bind _ashud_my_flying_shmup (cast `/Game/core/HUD_MyFlyingShmup` (`PlayerController.GetHUD` (`self.As Player Controller`))))
  (bind _playerwidget (`/Game/core/HUD_MyFlyingShmup.PlayerWidget` _ashud_my_flying_shmup))
  (`/Engine/EditorBlueprintResources/StandardMacros.IsValid` _playerwidget
    (:`Is Valid`
      (`/Game/core/BPI_MyFlyingShmup.SetHealthPercent` _playerwidget (`KismetMathLibrary.SafeDivide` (`self.Health`) (`self.MaxHealth`))))))

(fn `UserConstructionScript`)